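; Fireball gameplay ability that launches a homing-style projectile at the caster's selected target and applies burn damage.
; Activation captures the target, runs an interruptible cast, then net-syncs before committing.
; On commit, a projectile task flies to the captured target, cancelling if it is lost.
; On hit, after another net sync, the authority applies hit and periodic damage gameplay effects to the target's owner.
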(event `self.K2_ActivateAbility`
  ;[1 0.4097 0 0.416] Casting section
  (`self.SetCapturedTarget` (`self.GetSelectedTarget`))
  (`AbilityTask_Casting.WaitCasting` 1.0 (struct) (struct :`TagName` "Character.State.Casting")
    (:`OnSuccess`
      (`AbilityTask_NetworkSyncPoint.WaitNetSync` "BothWait"
        (:`OnSync`
          (`self.K2_CommitAbility`))))
    (:`OnInterrupt`
      (`self.K2_CancelAbility`))))

(event `self.K2_CommitExecute`
  (bind _returnvalue (`AbilitySystemBlueprintLibrary.AbilityTargetDataFromActor` (`ActorComponent.GetOwner` (`self.GetCapturedTarget`))))
  ;[0.04168 0.01652 1 0.542] Projectile flight section
  (`AbilityTask_LaunchProjectile.LaunchProjectileToTarget` "/Game/Player/Abilities/Fireball/BP_FireBall_FX.BP_FireBall_FX_C" (`self.GetCapturedTarget`) 3000.0 0.0
    (:`OnHit`
      (`AbilityTask_NetworkSyncPoint.WaitNetSync` "BothWait"
        (:`OnSync`
          (`self.K2_HasAuthority`
            (:`True`
              ;[1 0 0 0.531] Apply effects
              (`self.BP_ApplyGameplayEffectToTarget` _returnvalue "/Game/Player/Abilities/Fireball/BP_FireBall_HitDamage.BP_FireBall_HitDamage_C")
              (`self.BP_ApplyGameplayEffectToTarget` _returnvalue "/Game/Player/Abilities/Fireball/BP_FireBall_PeriodicDamage.BP_FireBall_PeriodicDamage_C"))))))
    (:`OnTargetLost`
      (`self.K2_CancelAbility`))
    (:`OnTaskDestroy`
      (`self.K2_EndAbility`))))

(fn `OnRep_NewEventDispatcher_0`)